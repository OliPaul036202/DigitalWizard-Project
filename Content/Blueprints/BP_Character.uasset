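; Player character Blueprint with jumping and a fireball charge, though only the Jump and Charge release handlers are live.
; Releasing Jump stops jumping unless WASD is held; releasing Charge stops the montage, then detaches and destroys any valid FireBall.
; Unconnected chains hold a cooldown-gated dash or jump, pause menu toggling, and fireball spawning, socket attachment and forward shooting.
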(event Input|ActionEvents|InputActionJump
  (params (Key :type Key%20Structure :default "None"))
  (bind _returnvalue (Game|GetPlayerController 0))
  (:Released
    (if (not (Math|Boolean|ORBoolean (Game|Player|IsInputKeyDown _returnvalue "W") (Game|Player|IsInputKeyDown _returnvalue "S") (Game|Player|IsInputKeyDown _returnvalue "A") (Game|Player|IsInputKeyDown _returnvalue "D")))
      (Character|StopJumping))))

(event Input|ActionEvents|InputActionPause
  (params (Key :type Key%20Structure :default "None"))
  ;[1 1 1] Pause/Unpause
)

(event Input|ActionEvents|InputActionCharge
  (params (Key :type Key%20Structure :default "None"))
  (:Released
    (Animation|StopAnimMontage 0)
    (Utilities|IsValid (.FireBall (Variables|Default|GetFireBall))
      (:Is%20Valid
        (Transformation|DetachFromActor (.FireBall (Variables|Default|GetFireBall)) "KeepWorld" "KeepWorld" "KeepWorld")
        (CallFunction|DestroyFireBall (.FireBall (Variables|Default|GetFireBall)))
        (Variables|Default|SetFireBall 0)))))

(event Input|ActionEvents|InputActionFire
  (params (Key :type Key%20Structure :default "None")))

(fn ConstructionScript)