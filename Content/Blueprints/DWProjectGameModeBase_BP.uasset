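; Game mode Blueprint that respawns the player's MainCharacter_BP after it is destroyed.
; On BeginPlay it casts player character 0 and binds OnDeath to its OnDestroyed event.
; OnDeath waits two seconds, spawns a replacement at the SpawnTransform variable, and has player controller 0 possess it.
; It then calls Respawn, which re-binds the death event to the new character so the cycle repeats.
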(event Custom|OnDeath
  (params (DestroyedActor :type Actor%20Object%20Reference))
  (Utilities|FlowControl|Delay 2.0)
  (bind _returnvalue (Game|SpawnActorfromClass "/Game/Blueprints/MainCharacter_BP.MainCharacter_BP_C" (Variables|Default|GetSpawn%20Transform) "Undefined" 0 0))
  (Pawn|Possess (Game|GetPlayerController 0) _returnvalue)
  (CallFunction|Respawn))

(event Custom|Respawn
  (bind _asmain_character_bp (Utilities|Casting|CastToMainCharacter_BP (Game|GetPlayerCharacter 0)))
  (Game|BindEventtoOnDestroyed _asmain_character_bp (delegate Custom|OnDeath)))

(event EventBeginPlay
  (bind _asmain_character_bp (Utilities|Casting|CastToMainCharacter_BP (Game|GetPlayerCharacter 0)))
  (Game|BindEventtoOnDestroyed _asmain_character_bp (delegate Custom|OnDeath)))

(event EventTick
  (params (DeltaSeconds :type Float%20%28single-precision%29)))

(fn ConstructionScript)