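; BP_Magic_Door is a hidden wall door that opens once enough collectables have been gathered.
; When the main character overlaps its collision volume, it reads TotalCollectables from the game mode and checks it against a threshold.
; If met, a timeline moves the wall's relative location; otherwise a hint message prints on screen.
; The end-overlap event only casts the character and does nothing further.
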(event OnComponentBeginOverlap(Collision)
  (params (OverlappedComponent :type Primitive%20Component%20Object%20Reference) (OtherActor :type Actor%20Object%20Reference) (OtherComp :type Primitive%20Component%20Object%20Reference) (OtherBodyIndex :type Integer) (bFromSweep :type Boolean) (SweepResult :type Hit%20Result%20Structure%20%28by%20ref%29))
  (Utilities|Casting|CastToMainCharacter_BP OtherActor)
  (bind _asdwproject_game_mode_base_bp (Utilities|Casting|CastToDWProjectGameModeBase_BP (Game|GetGameMode)))
  (if (>= (Variables|/Game/Blueprints/DWProjectGameModeBase_BP.DWProjectGameModeBase_BP_C|GetTotal%20Collectables _asdwproject_game_mode_base_bp) 3)
    (bind _open_track (Timeline|Open%20Door Play)
      (:Update
        (Transformation|SetRelativeLocation (Variables|Default|GetWall) _open_track false false)))
    (else
      (Development|PrintString "\"You sense something's off will this wall\"" true true "(R=1.000000,G=0.293800,B=0.000000,A=1.000000)" 4.0))))

(event OnComponentEndOverlap(Collision)
  (params (OverlappedComponent :type Primitive%20Component%20Object%20Reference) (OtherActor :type Actor%20Object%20Reference) (OtherComp :type Primitive%20Component%20Object%20Reference) (OtherBodyIndex :type Integer))
  (Utilities|Casting|CastToMainCharacter_BP OtherActor))

(fn ConstructionScript)