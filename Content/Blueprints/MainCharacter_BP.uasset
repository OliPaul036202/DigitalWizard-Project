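; Player mage character that turns to face the mouse cursor each tick via a trace and tracks clamped health.
; Jump becomes a launch-based dash while WASD is held.
; Charge spawns a fireball on the magic socket, Shoot fires it forward, and releasing Charge destroys an unfired one.
; E and Q spawn damage and heal AoEs from cursor traces; these and dash use flag-gated DoOnce/Delay cooldowns, while pause logic is unwired.
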(event EventBeginPlay
  ;[1 1 1] Show Mouse
  (Variables|/Script/Engine.PlayerController|SetbShowMouseCursor (Game|GetPlayerController 0) true)
  (Variables|Default|SetCurrentHealth (Variables|Default|GetMaxHealth)))

(event EventTick
  (params (DeltaSeconds :type Float%20%28single-precision%29))
  (bind _returnvalue (Game|GetPlayerController 0))
  (bind (_worldlocation _worlddirection) (Game|Player|ConvertMouseLocationToWorldSpace _returnvalue))
  (bind _outhit (Collision|LineTraceByChannel _worldlocation (+ (* _worlddirection 5e+04) _worlddirection) "TraceTypeQuery1" false 0 "None"))
  (Transformation|SetActorRotation (Math|Rotator|MakeRotator 0.0 0.0 (.yaw (Math|Rotator|FindLookatRotation (Transformation|GetActorLocation) (Math|Vector|MakeVector (.x (.Location (Collision|BreakHitResult _outhit))) (.y (.Location (Collision|BreakHitResult _outhit))) 0.0))))))

(event EventDamage
  (params (Amount :type Float%20%28single-precision%29))
  ;[1 1 1] Damage
  (Variables|Default|SetCurrentHealth (Math|Float|Clamp(Float) (- (Variables|Default|GetCurrentHealth) Amount) 0.0 (Variables|Default|GetMaxHealth))))

(event EventHeal
  (params (Amount :type Float%20%28single-precision%29))
  ;[1 1 1] Heal
  (Variables|Default|SetCurrentHealth (Math|Float|Clamp(Float) (+ (Variables|Default|GetCurrentHealth) Amount) 0.0 (Variables|Default|GetMaxHealth))))

(event Input|ActionEvents|InputActionJump
  (params (Key :type Key%20Structure :default "None"))
  (bind _returnvalue (Game|GetPlayerController 0))
  (bind _returnvalue_2 (Game|Player|IsInputKeyDown _returnvalue "W"))
  (bind _returnvalue_3 (Game|Player|IsInputKeyDown _returnvalue "S"))
  (bind _returnvalue_4 (Game|Player|IsInputKeyDown _returnvalue "A"))
  (bind _returnvalue_5 (Game|Player|IsInputKeyDown _returnvalue "D"))
  (bind _returnvalue_6 (Math|Boolean|ORBoolean _returnvalue_2 _returnvalue_3 _returnvalue_4 _returnvalue_5))
  ;[1 1 1] Dash
  (:Pressed
    (if _returnvalue_6
      (if (Variables|Default|GetCan%20Dash?)
        (Utilities|FlowControl|DoOnce false :!label _label
          (:Completed
            (Character|LaunchCharacter "0, 0,200.000000" false false)
            (Utilities|FlowControl|Delay 0.1)
            (Character|LaunchCharacter (* (Math|Vector|GetForwardVector (Transformation|GetActorRotation)) 1e+03) false false)
            (Animation|PlayAnimMontage 0 1.0 "None")
            (Utilities|FlowControl|Delay 1.0)
            (goto _label Reset))))
      (else
        (Character|Jump))))
  (:Released
    (if (not _returnvalue_6)
      (Character|StopJumping))))

(event Input|ActionEvents|InputActionPause
  (params (Key :type Key%20Structure :default "None"))
  ;[1 1 1] Pause/Unpause
)

(event Input|ActionEvents|InputActionCharge
  (params (Key :type Key%20Structure :default "None"))
  ;[1 1 1] Cast Fire Ball
  (:Pressed
    (bind _returnvalue (Game|SpawnActorfromClass "/Game/Blueprints/BP_FireBall.BP_FireBall_C" (Math|Transform|MakeTransform "0, 0, 0" (Math|Conversions|RotationFromXVector (Transformation|GetActorForwardVector)) "1,1,1") "AdjustIfPossibleButAlwaysSpawn" 0 0))
    (bind _output_get (Variables|Default|SetFireBall _returnvalue))
    (Transformation|AttachComponentToComponent _output_get (Variables|Default|GetMagic%20Socket) "None" "SnapToTarget" "KeepWorld" "KeepWorld" true))
  (:Released
    (Animation|StopAnimMontage 0)
    (Utilities|IsValid (Variables|Default|GetFireBall)
      (:Is%20Valid
        (Transformation|DetachFromActor (Variables|Default|GetFireBall) "KeepWorld" "KeepWorld" "KeepWorld")
        (Default|DestroyFireBall (Variables|Default|GetFireBall))
        (Variables|Default|SetFireBall 0)))))

(event Input|ActionEvents|InputActionShoot
  (params (Key :type Key%20Structure :default "None"))
  ;[1 1 1] Shoot Fire Ball
  (:Pressed
    (Utilities|IsValid (Variables|Default|GetFireBall)
      (:Is%20Valid
        (Animation|Montage|PlayMontage (Variables|Character|GetMesh) 0
          (:then
            (Default|ShootFireBall (Variables|Default|GetFireBall) (Transformation|GetActorForwardVector) 5e+02)
            (Variables|Default|SetFireBall 0)))))))

(event Input|KeyboardEvents|Q
  (params (Key :type Key%20Structure :default "None"))
  (bind _returnvalue (Game|GetPlayerController 0))
  (bind (_worldlocation _worlddirection) (Game|Player|ConvertMouseLocationToWorldSpace _returnvalue))
  ;[1 1 1] Heal AoE
  (:Pressed
    (bind _outhit (Collision|LineTraceByChannel _worldlocation (+ _worldlocation (* _worlddirection 9.5e+02)) "TraceTypeQuery1" false 0 "None"))
    (if (Variables|Default|GetCan%20Heal)
      (Utilities|FlowControl|DoOnce false :!label _label
        (:Completed
          (Animation|PlayAnimMontage 0 1.0 "None")
          (Game|SpawnActorfromClass "/Game/Blueprints/BP_HealAOE.BP_HealAOE_C" (Math|Transform|MakeTransform (.TraceEnd (Collision|BreakHitResult _outhit)) "0, 0, 0" "1,1,1") "AlwaysSpawn" 0 0)
          (Utilities|FlowControl|Delay 4.0)
          (goto _label Reset))))))

(event Input|KeyboardEvents|E
  (params (Key :type Key%20Structure :default "None"))
  (bind _returnvalue (Game|GetPlayerController 0))
  ;[1 1 1] AoE Attack
  (:Pressed
    (bind _outhit (Collision|LineTraceByChannel (.WorldLocation (Game|Player|ConvertMouseLocationToWorldSpace _returnvalue)) (.traceend (.HitResult (Game|Player|GetHitResultUnderCursorbyChannel _returnvalue "TraceTypeQuery3" true))) "TraceTypeQuery3" false 0 "None"))
    (if (Variables|Default|GetCan%20Aoe)
      (Utilities|FlowControl|DoOnce false :!label _label
        (:Completed
          (Animation|PlayAnimMontage 0 1.0 "None")
          (Game|SpawnActorfromClass "/Game/Blueprints/BP_MagicAOE.BP_MagicAOE_C" (Math|Transform|MakeTransform (.TraceEnd (Collision|BreakHitResult _outhit)) "0, 0, 0" "1,1,1") "AlwaysSpawn" 0 0)
          (Utilities|FlowControl|Delay 4.0)
          (goto _label Reset))))))

(fn ConstructionScript)

(fn GetHealthasRatio
  (return (/ (Variables|Default|GetCurrentHealth) (Variables|Default|GetMaxHealth))))