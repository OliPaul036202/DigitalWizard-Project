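; BP_FireBall is a fireball projectile that is launched with a given direction and speed.
; On shoot, it detaches from its parent, sets the projectile movement velocity and facing, and switches the effect from summoning to trail through User parameters on MagicFX.
; After a fixed delay it destroys itself by deactivating the effect and setting a short lifespan, giving existing particles time to fade.
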(event Custom|Shoot%20Fire%20Ball
  (params (Direction :type Vector) (Speed :type Float%20%28single-precision%29))
  (bind _magic_fx (Variables|Default|GetMagic%20FX))
  (Transformation|DetachFromActor "KeepWorld" "KeepWorld" "KeepWorld")
  (Variables|/Script/Engine.MovementComponent|SetVelocity (Variables|Default|GetProjectileMovement) (* Direction Speed))
  (Transformation|SetActorRotation (Math|Conversions|RotationFromXVector Direction))
  (Niagara|SetNiagaraVariable(Float) _magic_fx "User.TrailRate" 1.0)
  (Niagara|SetNiagaraVariable(Float) _magic_fx "User.SummonRate" 0.0)
  (Utilities|FlowControl|Delay 2.0)
  (CallFunction|DestroyFireBall))

(event Custom|Destroy%20Fire%20Ball
  (Components|Activation|Deactivate (Variables|Default|GetMagic%20FX))
  (Actor|SetLifeSpan 2.0))

(fn ConstructionScript)