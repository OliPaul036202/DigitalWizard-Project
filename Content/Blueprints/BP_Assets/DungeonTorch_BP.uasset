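; DungeonTorch_BP is a dungeon torch actor that makes its point light flicker.
; On Tick, a random short delay precedes picking a new random intensity within a narrow high range.
; A timeline with a 0.05-second tick interval then eases the light from its current intensity to the new one using sinusoidal in-out interpolation.
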(event EventBeginPlay)

(event Collision|EventActorBeginOverlap
  (params (OtherActor :type Actor%20Object%20Reference)))

(event EventTick
  (params (DeltaSeconds :type Float%20%28single-precision%29))
  (Utilities|FlowControl|Delay (Math|Random|RandomFloatinRange 0.0 0.2))
  (Variables|Default|SetOldIntensity (Variables|/Script/Engine.LightComponentBase|GetIntensity (Variables|Default|GetPointLight)))
  (Variables|Default|SetNewIntensity (Math|Random|RandomFloatinRange 9.5e+03 1e+04))
  (Class|ActorComponent|SetComponentTickInterval (Variables|Default|GetFlicker%20Timeline) 0.05)
  (bind _alpha (Timeline|Flicker%20TImeline PlayFromStart)
    (:Update
      (Rendering|Components|Light|SetIntensity (Variables|Default|GetPointLight) (Math|Interpolation|Ease "SinusoidalInOut" _alpha (Variables|Default|GetOldIntensity) (Variables|Default|GetNewIntensity))))))

(fn ConstructionScript)