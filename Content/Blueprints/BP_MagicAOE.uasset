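; Short-lived magic area-of-effect actor that damages and knocks back enemies, destroying itself two seconds after spawning.
; On BeginPlay it asks GS_ThirdPerson for a line-of-sight AOE instigated by the player, whose hit callback sends DamageMessage to each hit actor.
; Separately, sphere overlaps cast to Mimic, standard or red slime enemies, subtract Damage directly from their health and launch them opposite their facing.
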(event OnComponentBeginOverlap(Sphere)
  (params (OverlappedComponent :type Primitive%20Component%20Object%20Reference) (OtherActor :type Actor%20Object%20Reference) (OtherComp :type Primitive%20Component%20Object%20Reference) (OtherBodyIndex :type Integer) (bFromSweep :type Boolean) (SweepResult :type Hit%20Result%20Structure%20%28by%20ref%29))
  (bind _asmimic_enemy_bp (Utilities|Casting|CastToMimicEnemy_BP OtherActor)
    (:then
      (Variables|/Script/DWProject.Enemy|SetCurrentHealthEnemy _asmimic_enemy_bp (- (Variables|/Script/DWProject.Enemy|GetCurrentHealthEnemy _asmimic_enemy_bp) (Variables|Default|GetDamage)))
      (Character|LaunchCharacter _asmimic_enemy_bp (* (Transformation|GetActorForwardVector _asmimic_enemy_bp) -2e+03) false false))
    (:CastFailed
      (bind _asenemy_bp (Utilities|Casting|CastToEnemy_BP OtherActor)
        (:then
          (Variables|/Script/DWProject.Enemy|SetCurrentHealthEnemy _asenemy_bp (- (Variables|/Script/DWProject.Enemy|GetCurrentHealthEnemy _asenemy_bp) (Variables|Default|GetDamage)))
          (Character|LaunchCharacter _asenemy_bp (Math|Vector|MakeVector (.x (* (Transformation|GetActorForwardVector _asenemy_bp) -1.5e+03)) (.y (* (Transformation|GetActorForwardVector _asenemy_bp) -1.5e+03)) 2e+02) false false))
        (:CastFailed
          (bind _asslime_enemy_red_bp (Utilities|Casting|CastToSlimeEnemyRed_BP OtherActor))
          (Variables|/Script/DWProject.Enemy|SetCurrentHealthEnemy _asslime_enemy_red_bp (- (Variables|/Script/DWProject.Enemy|GetCurrentHealthEnemy _asslime_enemy_red_bp) (Variables|Default|GetDamage)))
          (Character|LaunchCharacter _asslime_enemy_red_bp (Math|Vector|MakeVector (.x (* (Transformation|GetActorForwardVector _asslime_enemy_red_bp) -1.5e+03)) (.y (* (Transformation|GetActorForwardVector _asslime_enemy_red_bp) -1.5e+03)) 2e+02) false false))))))

(event OnComponentHit(Sphere)
  (params (HitComponent :type Primitive%20Component%20Object%20Reference) (OtherActor :type Actor%20Object%20Reference) (OtherComp :type Primitive%20Component%20Object%20Reference) (NormalImpulse :type Vector :default "0, 0, 0") (Hit :type Hit%20Result%20Structure%20%28by%20ref%29)))

(event Custom|CustomEvent_0
  (params (Hit%20Actor :type Actor%20Object%20Reference))
  (Class|HealthInterface|Damage(Message) Hit%20Actor 1e+01))

(event EventBeginPlay
  (bind _asgs_third_person (Utilities|Casting|CastToGS_ThirdPerson (Game|GetGameState)))
  (Default|SpawnAOE _asgs_third_person (Transformation|GetActorLocation) 2.8e+02 true (Game|GetPlayerCharacter 0) (delegate Custom|CustomEvent_0) 0.0 "(R=100.000000,G=0.000000,B=0.000000,A=1.000000)")
  (Utilities|FlowControl|Delay 2.0)
  (Actor|DestroyActor))

(fn ConstructionScript)